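; BP_ForceField is a shield dome spell actor that shows impacts on its surface and destroys itself after a short timer.
; Sphere hits create a dynamic material on Sphere1, set the impact position, and spawn shield particles along the hit normal.
; An Animate timeline drives the material's ripple radius and calls ForceFieldDestroyed on each update, which destroys the field if the hitting actor is a BP_Fireball.
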(event `self.ReceiveBeginPlay`
  (`KismetSystemLibrary.K2_SetTimerDelegate` (delegate `OnForceFieldExpire`) 5.0))

(event `OnForceFieldExpire`
  (`self.K2_DestroyActor` self))

(event `self.Sphere.OnComponentHit`
  (params (HitComponent :type "PrimitiveComponent Object Reference") (OtherActor :type "Actor Object Reference") (OtherComp :type "PrimitiveComponent Object Reference") (NormalImpulse :type "Vector Structure") (Hit :type "HitResult Structure (by ref)"))
  (bind _returnvalue (`PrimitiveComponent.CreateDynamicMaterialInstance` (`self.Sphere1`) 0 null "None"))
  (`MaterialInstanceDynamic.SetVectorParameterValue` _returnvalue "pos" (`KismetMathLibrary.Conv_VectorToLinearColor` Hit_ImpactPoint))
  (`GameplayStatics.SpawnEmitterAtLocation` "/Game/Spells/ShieldDome/PS_ShieldParticles.PS_ShieldParticles" Hit_ImpactPoint (`KismetMathLibrary.MakeRotFromX` Hit_Normal))
  (bind (_direction _newtrack_0) (`Timeline|Animate` :!via `PlayFromStart`)
    (:`Update`
      (`MaterialInstanceDynamic.SetScalarParameterValue` _returnvalue "radius" (* _newtrack_0 200.0))
      (`self.ForceFieldDestroyed` OtherActor))))

(event `ForceFieldDestroyed`
  (params (HitActor :type "Actor Object Reference"))
  (cast `/Game/Spells/Fireball/BP_Fireball` HitActor)
  (`self.K2_DestroyActor` self))

(fn `UserConstructionScript`)