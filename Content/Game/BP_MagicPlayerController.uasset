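; BP_MagicPlayerController is a player controller that handles team selection and spawn requests when a player joins.
; On BeginPlay, the authority possesses the first BP_MagicEmptyPawn it finds as a placeholder, while the local controller adds the WBP_TeamSelect widget to the viewport.
; The TeamSelected event passes the chosen team and this controller to BP_GameMode's RequestSpawn.
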(event `self.ReceiveBeginPlay`
  (`|ExecutionSequence`
    (:`then_0`
      (`/Engine/EditorBlueprintResources/ActorMacros.Switch Has Authority`
        (:`Authority`
          (bind _outactors (`GameplayStatics.GetAllActorsOfClass` "/Game/Game/BP_MagicEmptyPawn.BP_MagicEmptyPawn_C"))
          (`self.Possess` (`|GetArrayItem` _outactors)))))
    (:`then_1`
      (if (`self.IsLocalController`)
        (bind _returnvalue (`|CreateWidget` "/Game/UI/Menus/WBP_TeamSelect.WBP_TeamSelect_C"))
        (`UserWidget.AddToViewport` _returnvalue 0)))))

(event `TeamSelected`
  (params (Team :type "ETeams Enum" :default "None"))
  (bind _asbp_game_mode (cast `/Game/Game/BP_GameMode` (`GameplayStatics.GetGameMode`)))
  (`/Game/Game/BP_GameMode.RequestSpawn` _asbp_game_mode Team self))

(fn `UserConstructionScript`)